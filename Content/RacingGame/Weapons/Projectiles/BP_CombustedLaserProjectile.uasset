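; BP_CombustedLaserProjectile is a racing-game laser projectile that travels along the track spline.
; On BeginPlay it caches the BP_Track actor.
; Each tick it advances a distance by ForwardVelocity and delta time, snaps the root to that spline point, and orients it to the spline direction closest to the projectile.
; SetProjectileMaterial applies a given laser material to the projectile.
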(event `self.ReceiveBeginPlay`
  ;[1 1 1] save track as variable
  (bind _returnvalue (`GameplayStatics.GetActorOfClass` "/Game/RacingGame/Track/BP_Track.BP_Track_C"))
  (set `self.Track` _returnvalue))

(event `self.ReceiveTick`
  (params (DeltaSeconds :type "Float (single-precision)"))
  (bind _spline (`/Game/RacingGame/Track/BP_Track.Spline` (`self.Track`)))
  (`|ExecutionSequence`
    (:`then_0`
      ;[1 1 1] Calculate rotation
      (`/Engine/EditorBlueprintResources/StandardMacros.IsValid` _spline
        (:`Is Valid`
          (set `self.UpdateRotation` (`KismetMathLibrary.MakeRotFromX` (`SplineComponent.FindDirectionClosestToWorldLocation` _spline (`SceneComponent.K2_GetComponentLocation` (`self.Projectile`)) "World"))))))
    (:`then_1`
      ;[1 1 1] Calculate distance along track
      (set `self.TrackPosition` (+ (* (`self.ForwardVelocity`) (`GameplayStatics.GetWorldDeltaSeconds`)) (`self.TrackPosition`))))
    (:`then_2`
      ;[1 1 1] Update movement
      (`SceneComponent.K2_SetWorldLocationAndRotation` (`self.RootComponent`) (`SplineComponent.GetLocationAtDistanceAlongSpline` (`/Game/RacingGame/Track/BP_Track.Spline` (`self.Track`)) (`self.TrackPosition`) "World") (`self.UpdateRotation`) false false))))

(fn `SetProjectileMaterial`
  (params (LaserMaterial :type "MaterialInstance Object Reference"))
  (`PrimitiveComponent.SetMaterial` (`self.Projectile`) 0 LaserMaterial))

(fn `UserConstructionScript`)