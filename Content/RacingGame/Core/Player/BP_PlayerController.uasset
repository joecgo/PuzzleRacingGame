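; Player controller for the racing game that caches HUD, game state and the possessed vehicle, and handles engineer grid input, cheats and boost-pad feedback.
; Engineer inputs rotate or combust the block under the HUD cursor through the game state, with timer-throttled grid navigation.
; Tick follows the game state's ground shape, switching between the vehicle's full-pipe and half-pipe cameras, blending on shape changes.
; Boost hits trigger sound, rumble, camera shake and HUD points.
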(event `self.ReceivePossess`
  (params (PossessedPawn :type "Pawn Object Reference"))
  (`|ExecutionSequence`
    (:`then_0`
      ;[1 1 1] save HUD reference
      (bind _asbp_hud (cast `/Game/RacingGame/UI/BP_HUD` (`self.GetHUD`)))
      (set `self.HUD` _asbp_hud))
    (:`then_1`
      ;[1 1 1] Save game state ref
      (bind _asbp_game_state (cast `/Game/RacingGame/Core/GameStates/BP_GameState` (`GameplayStatics.GetGameState`)))
      (set `self.GameState` _asbp_game_state))
    (:`then_2`
      ;[1 1 1] save ref to controlled vehicle and save player index
      (bind _asbp_vehicle (cast `/Game/RacingGame/Vehicles/BP_Vehicle` PossessedPawn))
      (bind _output_get (set `self.ControlledVehicle` _asbp_vehicle))
      (set `self.PlayerIndex` (`/Game/RacingGame/Vehicles/BP_Vehicle.PlayerIndex` _output_get)))))

(event `Key|Gamepad_Special_Left`
  (params (Key :type "Key Structure"))
  ;[1 1 1] Cheats
  (:`Pressed`
    (bind _asbp_cheat_manager (cast `/Game/RacingGame/Core/Cheats/BP_CheatManager` (`self.CheatManager`) :!label _label))
    (`/Game/RacingGame/Core/Cheats/BP_CheatManager.DamagePlayer` _asbp_cheat_manager)))

(event `Key|C`
  (params (Key :type "Key Structure"))
  ;[1 1 1] Cheats
  (:`Pressed`
    (goto _label)))

(event `HitBoostPad`
  (params (VehicleVelocity :type "Float (double-precision)"))
  ;[1 1 1] boost feedback
  (`GameplayStatics.PlaySound2D` "/Game/RacingGame/Audio/SFX/BoostHit.BoostHit" 1.5 VehicleVelocity 0.0 null null)
  (`self.PlayDynamicForceFeedback` 1.0 0.15)
  (`self.Score Points to HUD`)
  (`GameplayStatics.PlayWorldCameraShake` "/Game/RacingGame/Camera/Shakes/CameraShake_ShortHit.CameraShake_ShortHit_C" (0.0 0.0 0.0) 999999995904.0 999999995904.0 0.0))

(event `InputAction|GridBlockRotateClockwise`
  (params (Key :type "Key Structure"))
  ;[1 1 1] Engineer input
  (:`Pressed`
    (bind (_column _row) (`/Game/RacingGame/UI/BP_HUD.GetCursorPosition` (`self.HUD`)))
    (`/Game/RacingGame/Core/GameStates/BP_GameState.RotateBlock` (`self.GameState`) _column _row true)))

(event `InputAction|GridBlockRotateCounterClockwise`
  (params (Key :type "Key Structure"))
  ;[1 1 1] Engineer input
  (:`Pressed`
    (bind (_column _row) (`/Game/RacingGame/UI/BP_HUD.GetCursorPosition` (`self.HUD`)))
    (`/Game/RacingGame/Core/GameStates/BP_GameState.RotateBlock` (`self.GameState`) _column _row false)))

(event `InputAction|CombustSystem`
  (params (Key :type "Key Structure"))
  ;[1 1 1] Engineer input
  (:`Pressed`
    (bind (_column _row) (`/Game/RacingGame/UI/BP_HUD.GetCursorPosition` (`self.HUD`)))
    (`/Game/RacingGame/Core/GameStates/BP_GameState.CombustSystemEvent` (`self.GameState`) _column _row)))

(event `self.ReceiveTick`
  (params (DeltaSeconds :type "Float (single-precision)"))
  (bind _controlledvehicle (`self.ControlledVehicle`))
  (`|ExecutionSequence`
    (:`then_0`
      ;[1 1 1] Select the desired view target from the anchor vehicle
      (set `self.DesiredViewTarget` (select `/Game/RacingGame/Core/DataTypes/GroundShape` (`self.DesiredGroundShape`) :`NewEnumerator0` (`ChildActorComponent.ChildActor` (`/Game/RacingGame/Vehicles/BP_Vehicle.Camera_FullPipe` _controlledvehicle)) :`NewEnumerator1` (`ChildActorComponent.ChildActor` (`/Game/RacingGame/Vehicles/BP_Vehicle.Camera_HalfPipe` _controlledvehicle)))))
    (:`then_1`
      ;[1 1 1] Set desired ground shape for the view target (fullpipe vs halfpipe) --> check if there is a new view target --> blend to the new view target
      (bind _asbp_game_state (cast `/Game/RacingGame/Core/GameStates/BP_GameState` (`GameplayStatics.GetGameState`)))
      (set `self.DesiredGroundShape` (`/Game/RacingGame/Core/GameStates/BP_GameState.GroundState` _asbp_game_state))
      (if (!= (`self.GetViewTarget`) (`self.DesiredViewTarget`))
        (`self.SetViewTargetWithBlend` (`self.DesiredViewTarget`) (`KismetMathLibrary.SelectFloat` 1.0 0.0 (`|EnumInequality` (`self.DesiredGroundShape`) (`self.ViewTargetGroundShape`))) "VTBlend_EaseInOut" 2.0)
        (set `self.ViewTargetGroundShape` (`self.DesiredGroundShape`))))
    (:`then_2`
      ;[1 1 1] Manage grid nav rate and navigate grid if not on cooldown
      (if (> (+ (`KismetMathLibrary.Abs` (`self.GetInputAxisValue`)) (`KismetMathLibrary.Abs` (`self.GetInputAxisValue`))) 0.0)
        (if (`self.GridNavReady`)
          (set `self.GridNavReady` false)
          (`KismetSystemLibrary.K2_SetTimer` null "SetGridNavReady" (`self.GridNavRate`))
          (`/Game/RacingGame/UI/BP_HUD.GridNavigation` (`self.HUD`) (`KismetMathLibrary.MakeVector2D` (`self.GetInputAxisValue`) (`self.GetInputAxisValue`))))
        (else
          (`self.SetGridNavReady`))))))

(fn `Score Points to HUD`
  (bind _asbp_hud (cast `/Game/RacingGame/UI/BP_HUD` (`self.GetHUD`)))
  (`/Game/RacingGame/UI/BP_HUD.ScorePoints` _asbp_hud (`self.HitBoostPoints`) (`self.PlayerIndex`)))

(fn `SetGridNavReady`
  (set `self.GridNavReady` true))

(fn `UserConstructionScript`)