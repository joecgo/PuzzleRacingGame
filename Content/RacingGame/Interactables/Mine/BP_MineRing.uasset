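; BP_MineRing is a racing game obstacle that arranges BP_Mine hazards in a spinning ring around its forward axis.
; The construction script spawns the mines as child actors at random rotations, spaced evenly by count and radius for the Full Circle layout.
; Tick rotates the whole actor clockwise or counterclockwise at a constant rate by continually interpolating toward a 90-degree offset.
; A DisableMines flag turns off both spawning and rotation.
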(event `self.ReceiveTick`
  (params (DeltaSeconds :type "Float (single-precision)"))
  (bind _returnvalue (`self.K2_GetActorRotation`))
  (bind _returnvalue_2 (`self.GetActorForwardVector`))
  (if (not (`self.bDisableMines`))
    (`self.K2_SetActorRelativeRotation` (`KismetMathLibrary.RInterpTo_Constant` _returnvalue (`KismetMathLibrary.ComposeRotators` _returnvalue (`KismetMathLibrary.SelectRotator` (`KismetMathLibrary.RotatorFromAxisAndAngle` _returnvalue_2 -90.0) (`KismetMathLibrary.RotatorFromAxisAndAngle` _returnvalue_2 90.0) (`self.bRotateClockwise`))) DeltaSeconds (`self.RotationRate`)))))

(fn `UserConstructionScript`
  (if (not (`self.bDisableMines`))
    (for _index (range (`self.MineCount`))
      (set `self.Index` _index)
      (switch `/Game/RacingGame/Core/DataTypes/SpawnPattern` "NewEnumerator0"
        (:`NewEnumerator0`
          ;[1 1 1] Full Circle Spawning
          (bind _returnvalue (`AddComponent|NODE_AddChildActorComponent-0` :`RelativeTransform` (`KismetMathLibrary.MakeTransform` (`KismetMathLibrary.RotateAngleAxis` (`KismetMathLibrary.MakeVector` 0.0 0.0 (`self.RingRadius`)) (* (`KismetMathLibrary.Conv_IntToDouble` (`self.Index`)) (/ 360.0 (`KismetMathLibrary.Conv_IntToDouble` (`self.MineCount`)))) (1.0 0.0 0.0)) (`KismetMathLibrary.RandomRotator` true))))
          (`ChildActorComponent.SetChildActorClass` _returnvalue "/Game/RacingGame/Interactables/Mine/BP_Mine.BP_Mine_C"))))))