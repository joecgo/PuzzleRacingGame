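; BP_Mine is a racing-game mine that explodes and destroys itself when any actor overlaps it.
; The overlap spawns a BP_ky_hit2 effect for pawns, with the pawn as instigator, or BP_ky_hit1 for other actors, each with its own scale variable.
; After the destroy call, a player-controlled pawn triggers PlayerDamaged on BP_GameState, with no damage applied here directly.
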(event `self.ReceiveActorBeginOverlap`
  (params (OtherActor :type "Actor Object Reference"))
  (bind _returnvalue (`SceneComponent.K2_GetComponentToWorld` (`self.DefaultSceneRoot`)))
  (`|ExecutionSequence`
    (:`then_0`
      ;[1 1 1] create mine explosion effect, collision with vehicle
      (bind _aspawn (cast `Pawn` OtherActor)
        (:`then`
          (bind _returnvalue_2 (`|SpawnActorFromClass` "/Game/FXVarietyPack/Blueprints/BP_ky_hit2.BP_ky_hit2_C" _returnvalue "AlwaysSpawn" "OverrideRootScale" null _aspawn))
          (`self.SetActorScale3D` _returnvalue_2 (`self.ExplosionScale_Projectile`)))
        (:`CastFailed`
          (bind _returnvalue_3 (`|SpawnActorFromClass` "/Game/FXVarietyPack/Blueprints/BP_ky_hit1.BP_ky_hit1_C" _returnvalue "AlwaysSpawn" "OverrideRootScale" null null))
          (`self.SetActorScale3D` _returnvalue_3 (`self.ExplosionScale_Vehicle`)))))
    (:`then_1`
      ;[1 1 1] destroy on impact with vehicle
      (`self.K2_DestroyActor`))
    (:`then_2`
      ;[1 1 1] if pawn is player controlled, report to game state that player was damaged
      (bind _aspawn_2 (cast `Pawn` OtherActor))
      (if (`Pawn.IsPlayerControlled` _aspawn_2)
        (bind _asbp_game_state (cast `/Game/RacingGame/Core/GameStates/BP_GameState` (`GameplayStatics.GetGameState`)))
        (`/Game/RacingGame/Core/GameStates/BP_GameState.PlayerDamaged` _asbp_game_state)))))

(fn `UserConstructionScript`)