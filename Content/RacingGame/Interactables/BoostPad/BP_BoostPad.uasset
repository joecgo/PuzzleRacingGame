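; BP_BoostPad is a single-use racing boost pad that triggers when a BP_Vehicle overlaps it.
; The first hit calls HitBoostPad on the vehicle, then BoostHit sets PlayerInteracted and swaps the decal to a red material to show it is used up.
; BoostHit also calls CollectBlockRandom on BP_GameState to give the player a random block.
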(event `self.ReceiveActorBeginOverlap`
  (params (OtherActor :type "Actor Object Reference"))
  ;[1 1 1] if boost isnt used up, send boost event to vehicle and self
  (bind _asbp_vehicle (cast `/Game/RacingGame/Vehicles/BP_Vehicle` OtherActor))
  (if (not (`self.PlayerInteracted`))
    (`/Game/RacingGame/Vehicles/BP_Vehicle.HitBoostPad` _asbp_vehicle)
    (`self.BoostHit`)))

(event `BoostHit`
  ;[1 1 1] boost hit
  (set `self.PlayerInteracted` true)
  (`self.Set Boost Color`)
  ;[1 1 1] Boost gives player a random block
  (bind _asbp_game_state (cast `/Game/RacingGame/Core/GameStates/BP_GameState` (`GameplayStatics.GetGameState`)))
  (`/Game/RacingGame/Core/GameStates/BP_GameState.CollectBlockRandom` _asbp_game_state))

(fn `Set Boost Color`
  (locals (bLocalAllPlayersInteracted :type Boolean :default true))
  (`DecalComponent.SetDecalMaterial` (`self.Decal`) "/Game/RacingGame/Interactables/BoostPad/MI_BoostPadDecal_Red.MI_BoostPadDecal_Red"))

(fn `UserConstructionScript`)