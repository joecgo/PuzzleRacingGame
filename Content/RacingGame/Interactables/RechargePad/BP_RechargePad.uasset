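; BP_RechargePad is a racing-game pad that recharges a BP_Vehicle while it overlaps the actor.
; Begin and end overlap call StartRecharging and StopRecharging, which notify both the vehicle and BP_GameState.
; A single RechargeActive flag gates both calls, so the pad tracks one recharge state rather than individual vehicles.
; SetBoostColor swaps the decal to a red boost-pad material but is not called within this Blueprint.
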(event `self.ReceiveActorEndOverlap`
  (params (OtherActor :type "Actor Object Reference"))
  ;[1 1 1] player exit recharge
  (bind _asbp_vehicle (cast `/Game/RacingGame/Vehicles/BP_Vehicle` OtherActor))
  (if (`self.RechargeActive`)
    (`self.StopRecharging` _asbp_vehicle)))

(event `self.ReceiveActorBeginOverlap`
  (params (OtherActor :type "Actor Object Reference"))
  ;[1 1 1] player entered recharge
  (bind _asbp_vehicle (cast `/Game/RacingGame/Vehicles/BP_Vehicle` OtherActor))
  (if (not (`self.RechargeActive`))
    (`self.StartRecharging` _asbp_vehicle)))

(fn `Set Boost Color`
  (locals (bLocalAllPlayersInteracted :type Boolean :default true))
  (`DecalComponent.SetDecalMaterial` (`self.Decal`) "/Game/RacingGame/Interactables/BoostPad/MI_BoostPadDecal_Red.MI_BoostPadDecal_Red"))

(fn `StartRecharging`
  (params (Vehicle :type "/Game/RacingGame/Vehicles/BP_Vehicle Object Reference"))
  (`/Game/RacingGame/Vehicles/BP_Vehicle.StartRecharingEvent` Vehicle)
  (set `self.RechargeActive` true)
  (bind _asbp_game_state (cast `/Game/RacingGame/Core/GameStates/BP_GameState` (`GameplayStatics.GetGameState`)))
  (`/Game/RacingGame/Core/GameStates/BP_GameState.StartRechargingEvent` _asbp_game_state))

(fn `StopRecharging`
  (params (Vehicle :type "/Game/RacingGame/Vehicles/BP_Vehicle Object Reference"))
  (`/Game/RacingGame/Vehicles/BP_Vehicle.StopRechargingEvent` Vehicle)
  (set `self.RechargeActive` false)
  (bind _asbp_game_state (cast `/Game/RacingGame/Core/GameStates/BP_GameState` (`GameplayStatics.GetGameState`)))
  (`/Game/RacingGame/Core/GameStates/BP_GameState.StopRechargingEvent` _asbp_game_state))

(fn `UserConstructionScript`)