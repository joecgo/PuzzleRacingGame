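; Racing track actor that builds its road mesh along an editable spline, either open or as a closed loop.
; The construction script rebuilds one shadowless spline mesh per segment, wrapping the last segment to the first point on loops.
; Each segment takes its up vector from the spline midpoint and derives start and end roll relative to that rotation.
; It also provides segment hiding by zero scale, scale reset on BeginPlay, and player start distance selection.
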(event `self.ReceiveBeginPlay`
  (`self.Reset Track Scale`))

(fn `ConstructTrackMesh`
  (locals (LocalCurrentTrackPoint :type Integer) (LocalNextTrackPoint :type Integer) (LocalCurrentSplineMesh :type "SplineMeshComponent Object Reference") (LocalTrackElementMesh :type "StaticMesh Object Reference" :default "StaticMesh'/Game/RacingGame/Track/S_OpenPipe.S_OpenPipe'") (LocalSplineMeshUpVector :type "Vector Structure") (LocalStartRoll :type "Float (double-precision)") (LocalEndRoll :type "Float (double-precision)") (LocalSplineMeshRotation :type "Rotator Structure"))
  (bind _spline (`self.Spline`))
  (bind _distance (`self.GetAverageDistanceBetweenSplinePoints` (`local.LocalCurrentTrackPoint`) (`local.LocalNextTrackPoint`) (`self.Spline`)))
  (bind (_startpoint _starttangent _endpoint _endtangent) (`self.GetSplineSegmentStartAndEnd` (`local.LocalCurrentTrackPoint`) (`local.LocalNextTrackPoint`)))
  ;[1 1 1] Set up loop for spline points, check for if this is a closed loop
  (for _array_element (`self.SplineMeshes`)
    (`ActorComponent.K2_DestroyComponent` _array_element))
  (`KismetArrayLibrary.Array_Clear` (`self.SplineMeshes`))
  (`SplineComponent.SetClosedLoop` (`self.Spline`) (`self.bIsClosedLoop`) true)
  (for _index (range (+ (- (`SplineComponent.GetNumberOfSplinePoints` (`self.Spline`)) (`KismetMathLibrary.SelectInt` 1 2 (`SplineComponent.IsClosedLoop` (`self.Spline`)))) 1))
    (set `local.LocalCurrentTrackPoint` _index)
    (set `local.LocalNextTrackPoint` (+ _index 1))
    (`|ExecutionSequence`
      (:`then_0`
        ;[1 1 1] Get the up vector for the spline mesh
        (set `local.LocalSplineMeshUpVector` (`SplineComponent.GetUpVectorAtDistanceAlongSpline` _spline _distance "Local"))
        (set `local.LocalSplineMeshRotation` (`SplineComponent.GetRotationAtDistanceAlongSpline` _spline _distance "Local")))
      (:`then_1`
        ;[1 1 1] Store the start roll
        (set `local.LocalStartRoll` (`KismetMathLibrary.MultiplyByPi` (/ (`self.GetRelativeRollAtSplinePoint` (`self.Spline`) (`local.LocalCurrentTrackPoint`) (`local.LocalSplineMeshRotation`)) 180.0)))
        ;[1 1 1] Store the end roll
        (set `local.LocalEndRoll` (`KismetMathLibrary.MultiplyByPi` (/ (`self.GetRelativeRollAtSplinePoint` (`self.Spline`) (`local.LocalNextTrackPoint`) (`local.LocalSplineMeshRotation`)) 180.0))))
      (:`then_2`
        ;[1 1 1] Generate spline mesh component
        (bind _returnvalue (`AddComponent|NODE_AddSplineMeshComponent-0`))
        (set `local.LocalCurrentSplineMesh` _returnvalue)
        (`StaticMeshComponent.SetStaticMesh` (`local.LocalCurrentSplineMesh`) (`local.LocalTrackElementMesh`))
        (`PrimitiveComponent.SetCastShadow` (`local.LocalCurrentSplineMesh`) false)
        (`SplineMeshComponent.SetSplineUpDir` (`local.LocalCurrentSplineMesh`) (`local.LocalSplineMeshUpVector`) true)
        (`SplineMeshComponent.SetStartAndEnd` (`local.LocalCurrentSplineMesh`) _startpoint _starttangent _endpoint _endtangent true)
        (`SplineMeshComponent.SetStartRoll` (`local.LocalCurrentSplineMesh`) (`local.LocalStartRoll`) true)
        (`SplineMeshComponent.SetEndRoll` (`local.LocalCurrentSplineMesh`) (`local.LocalEndRoll`) true)
        (`SplineComponent.SetUpVectorAtSplinePoint` (`self.Spline`) (`local.LocalCurrentTrackPoint`) (`local.LocalSplineMeshUpVector`) "World" true)
        (`KismetArrayLibrary.Array_Add` (`self.SplineMeshes`) (`local.LocalCurrentSplineMesh`))))))

(fn `Get Player Start Distance`
  (returns (Distance :type "Float (double-precision)"))
  (return (`KismetMathLibrary.SelectFloat` (`self.TrackEditorStartDistance`) (`self.PlayerStartDistance`) (`self.bUseTrackEditorStartPosition`))))

(fn `GetRelativeRollAtSplinePoint`
  (params (Spline :type "SplineComponent Object Reference") (PointIndex :type Integer) (RelativeTo :type "Rotator Structure"))
  (returns (Roll :type "Float (double-precision)"))
  (bind _returnvalue_roll (`KismetMathLibrary.BreakRotator` (`KismetMathLibrary.MakeRotationFromAxes` (`KismetMathLibrary.LessLess_VectorRotator` (`SplineComponent.GetDirectionAtSplinePoint` Spline PointIndex "Local") RelativeTo) (`KismetMathLibrary.LessLess_VectorRotator` (`SplineComponent.GetRightVectorAtSplinePoint` Spline PointIndex "Local") RelativeTo) (`KismetMathLibrary.LessLess_VectorRotator` (`SplineComponent.GetUpVectorAtSplinePoint` Spline PointIndex "Local") RelativeTo))))
  (return _returnvalue_roll))

(fn `HideMesh`
  (params (Mesh :type "SplineMeshComponent Object Reference"))
  (`SplineMeshComponent.SetStartScale` Mesh (0.0 0.0) true)
  (`SplineMeshComponent.SetEndScale` Mesh (0.0 0.0) true)
  (`KismetSystemLibrary.PrintString` "shrunk"))

(fn `Reset Track Scale`
  (for _array_element (`self.SplineMeshes`)
    (`SplineMeshComponent.SetStartScale` _array_element (1.0 1.0) true)
    (`SplineMeshComponent.SetEndScale` _array_element (1.0 1.0) true)))

(fn `UserConstructionScript`
  (locals (LocalCurrentTrackPoint :type Integer) (LocalNextTrackPoint :type Integer) (LocalSplineMeshUpVector :type "Vector Structure") (LocalSplineMeshRotation :type "Rotator Structure") (LocalStartRoll :type "Float (double-precision)") (LocalCurrentSplineMesh :type "SplineMeshComponent Object Reference") (LocalTrackElementMesh :type "StaticMesh Object Reference" :default "StaticMesh'/Game/RacingGame/Track/S_OpenPipe.S_OpenPipe'") (LocalEndRoll :type "Float (double-precision)") (LocalSplinesMeshes :type "Array of SplineMeshComponent Object Reference"))
  (`self.ConstructTrackMesh`))