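; AI controller for the Locust enemy that starts its formation behavior and relays fire and roll commands to the pawn.
; Tick waits until game time passes FormationStartTime, then runs BT_Locust once.
; StartFiring fires a burst of shots through a delayed-loop macro, and Roll adds to the Locust's desired roll.
; The looping timer for repeated bursts is disconnected, leaving the startup delay with no effect.
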(event `self.ReceiveTick`
  (params (DeltaSeconds :type "Float (single-precision)"))
  (bind _shotsinitialstartdelay (`self.ShotsInitialStartDelay`))
  ;[1 1 1] start activities of formation -> firing loop
  (if (`self.IsTimeToStartFormation`)
    (set `self.bCompletedFormationSync` true)
    (`self.RunBehaviorTree` "/Game/RacingGame/Enemies/Locust/Behavior/BT_Locust.BT_Locust")
    (`KismetSystemLibrary.Delay` (`KismetMathLibrary.SelectFloat` (+ (/ (`self.ShotsInterval`) 2.0) _shotsinitialstartdelay) _shotsinitialstartdelay))))

(event `Event StartFiring`
  (bind _asbp_locust (cast `/Game/RacingGame/Enemies/Locust/BP_Locust` (`self.K2_GetPawn`)))
  (`self.ForLoopDelay` 1 (`self.ShootsPerInterval`) (`self.ShotRate`)
    (:`LoopBody`
      (`/Game/RacingGame/Enemies/Locust/BP_Locust.FireShot` _asbp_locust))))

(event `Event Roll`
  (params (RollToAdd :type "Float (double-precision)"))
  (bind _asbp_locust (cast `/Game/RacingGame/Enemies/Locust/BP_Locust` (`self.K2_GetPawn`)))
  (set `/Game/RacingGame/Enemies/Locust/BP_Locust.DesiredRoll` (+ (`/Game/RacingGame/Enemies/Locust/BP_Locust.DesiredRoll` _asbp_locust) RollToAdd) _asbp_locust))

(fn `IsTimeToStartFormation`
  (returns (bStartFormation :type Boolean))
  (return (and (not (`self.bCompletedFormationSync`)) (> (`KismetSystemLibrary.GetGameTimeInSeconds`) (`self.FormationStartTime`)))))

(fn `StartFiring`
  (`self.Event StartFiring`))

(fn `UserConstructionScript`)