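; Locust enemy for the racing game that flies along the track spline, holding a set spacing relative to the player's vehicle.
; Each tick it eases roll toward a desired angle and speed toward its target distance, then places itself on the spline rolled around the tangent.
; A timed intro raises top speed and shows an invulnerable material.
; FireShot spawns blue lasers, and ending overlap with player projectiles or mines destroys it.
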(event `self.ReceiveBeginPlay`
  ;[1 1 1] set up initial variables
  (`|ExecutionSequence`
    (:`then_0`
      (bind _playervehicle (`self.GetPlayerVehicle`))
      (set `self.PlayerVehicle` _playervehicle))
    (:`then_1`
      (bind _track (`self.GetTrack`))
      (set `self.Track` _track))
    (:`then_2`
      (set `self.TrackPosition` (- (`/Game/RacingGame/Vehicles/BP_Vehicle.Distance` (`self.PlayerVehicle`)) 1000.0)))
    (:`then_3`
      (set `self.ForwardVelocity` (`/Game/RacingGame/Vehicles/BP_Vehicle.ForwardVelocity` (`self.PlayerVehicle`))))
    (:`then_4`
      (`PrimitiveComponent.SetMaterialByName` (`self.S_Locust`) "sh3" "/Game/RacingGame/Enemies/Locust/Materials/M_Locust_Invulnerable.M_Locust_Invulnerable")
      (`KismetSystemLibrary.Delay` (`self.IntroBoostDuration`))
      (`PrimitiveComponent.SetMaterialByName` (`self.S_Locust`) "sh3" "/Game/RacingGame/Enemies/Locust/Materials/M_Locust.M_Locust"))
    (:`then_5`
      (set `self.MaxForwardVelocity` (* (`self.MaxForwardVelocity`) (`self.IntroMaxVelocityMultiplier`)))
      (`KismetSystemLibrary.Delay` (`self.IntroBoostDuration`))
      (set `self.MaxForwardVelocity` (/ (`self.MaxForwardVelocity`) (`self.IntroMaxVelocityMultiplier`))))))

(event `self.ReceiveTick`
  (params (DeltaSeconds :type "Float (single-precision)"))
  (bind _distance (`self.GetSplineDistance`))
  (bind _forwardaccelerationrate (`self.ForwardAccelerationRate`))
  (bind _desiredrollapproachangle (`self.DesiredRollApproachAngle`))
  (bind _desiredpositionapproachdistance (`self.DesiredPositionApproachDistance`))
  (bind _spline (`/Game/RacingGame/Track/BP_Track.Spline` (`self.Track`)))
  (bind _returnvalue (`KismetMathLibrary.MapRangeClamped` (- (`self.DesiredTrackPosition`) (`self.TrackPosition`)) (* -1.0 _desiredpositionapproachdistance) _desiredpositionapproachdistance -1.0 1.0))
  (bind _returnvalue_2 (`KismetMathLibrary.MapRangeClamped` (- (`self.DesiredRoll`) (`self.Roll`)) (* -1.0 _desiredrollapproachangle) _desiredrollapproachangle -1.0 1.0))
  (bind _returnvalue_3 (`KismetMathLibrary.NegateVector` (`SplineComponent.GetTangentAtDistanceAlongSpline` _spline _distance "World")))
  (`|ExecutionSequence`
    (:`then_0`
      ;[1 1 1] Calculate roll velocity
      (set `self.RollVelocity` (* (`|EaseFunction` "EaseIn" (`KismetMathLibrary.Abs` _returnvalue_2) 0.0 (* (`KismetMathLibrary.SignOfFloat` _returnvalue_2) (`self.MaxRollVelocity`)) 1.25) (`GameplayStatics.GetWorldDeltaSeconds`))))
    (:`then_1`
      ;[1 1 1] Calculate roll
      (set `self.Roll` (+ (`self.Roll`) (`self.RollVelocity`))))
    (:`then_2`
      ;[1 1 1] Calculate rotation
      (`/Engine/EditorBlueprintResources/StandardMacros.IsValid` _spline
        (:`Is Valid`
          (set `self.UpdateRotation` (`KismetMathLibrary.MakeRotFromXZ` _returnvalue_3 (`KismetMathLibrary.RotateAngleAxis` (`SplineComponent.GetUpVectorAtDistanceAlongSpline` _spline _distance "World") (`self.Roll`) _returnvalue_3))))))
    (:`then_3`
      ;[1 1 1] set desired position on track in relation to player
      (set `self.DesiredTrackPosition` (+ (`/Game/RacingGame/Vehicles/BP_Vehicle.Distance` (`self.PlayerVehicle`)) (`self.TargetForwardPlayerSpacing`))))
    (:`then_4`
      ;[1 1 1] set forward acceleration based on direction of desired position
      (set `self.ForwardAcceleration` (`KismetMathLibrary.SelectFloat` _forwardaccelerationrate (* _forwardaccelerationrate -1.0) (> (`self.DesiredTrackPosition`) (`self.TrackPosition`)))))
    (:`then_5`
      ;[1 1 1] Update forward velocity
      (set `self.ForwardVelocity` (`|EaseFunction` "EaseIn" (`KismetMathLibrary.Abs` _returnvalue) 0.0 (* (`KismetMathLibrary.SignOfFloat` _returnvalue) (`self.MaxForwardVelocity`)) 0.5)))
    (:`then_6`
      ;[1 1 1] Calculate distance along track
      (set `self.TrackPosition` (+ (* (`self.ForwardVelocity`) (`GameplayStatics.GetWorldDeltaSeconds`)) (`self.TrackPosition`))))
    (:`then_7`
      ;[1 1 1] Update movement
      (`SceneComponent.K2_SetWorldLocationAndRotation` (`self.RootComponent`) (`SplineComponent.GetLocationAtDistanceAlongSpline` (`/Game/RacingGame/Track/BP_Track.Spline` (`self.Track`)) (`self.GetSplineDistance`) "World") (`self.UpdateRotation`) false false))))

(event `self.ReceiveActorEndOverlap`
  (params (OtherActor :type "Actor Object Reference"))
  ;[1 1 1] projectile type check
  (cast `/Game/RacingGame/Weapons/Projectiles/BP_LaserProjectile` OtherActor
    (:`then`
      ;[1 1 1] create explosion effect, collision with player or projectile
      (bind _returnvalue (`|SpawnActorFromClass` "/Game/FXVarietyPack/Blueprints/BP_ky_hit2.BP_ky_hit2_C" (`SceneComponent.K2_GetComponentToWorld` (`self.Sphere`)) "AlwaysSpawn" "OverrideRootScale" null null :!label _label)))
    (:`CastFailed`
      (cast `/Game/RacingGame/Weapons/Projectiles/BP_CombustedLaserProjectile` OtherActor
        (:`then`
          (goto _label))
        (:`CastFailed`
          (cast `/Game/RacingGame/Interactables/Mine/BP_Mine` OtherActor)))))
  (`self.SetActorScale3D` _returnvalue (`self.ExplosionScale_Projectile`))
  (`self.K2_DestroyActor`))

(fn `FireShot`
  (bind (_shotoffset_x _shotoffset_y _shotoffset_z) (`KismetMathLibrary.BreakVector` (`self.ShotOffset`)))
  (bind (_returnvalue_location _returnvalue_rotation) (`KismetMathLibrary.BreakTransform` (`SceneComponent.K2_GetComponentToWorld` (`self.S_Locust`))))
  ;[1 1 1] create object with correct offset
  (bind _returnvalue (`|SpawnActorFromClass` "/Game/RacingGame/Weapons/Projectiles/BP_EnemyLaserProjectile.BP_EnemyLaserProjectile_C" (`KismetMathLibrary.MakeTransform` (+ (* (`KismetMathLibrary.GetRightVector` _returnvalue_rotation) _shotoffset_x) (* (`KismetMathLibrary.GetUpVector` _returnvalue_rotation) _shotoffset_y) (* (`KismetMathLibrary.GetForwardVector` _returnvalue_rotation) _shotoffset_z) _returnvalue_location) _returnvalue_rotation) "AlwaysSpawn" "OverrideRootScale" null null))
  ;[1 1 1] set properties
  (`/Game/RacingGame/Weapons/Projectiles/BP_EnemyLaserProjectile.SetProjectileMaterial` _returnvalue "/Game/RacingGame/Weapons/Projectiles/MI_LaserProjectile_Blue.MI_LaserProjectile_Blue")
  (`self.SetLifeSpan` 6.0))

(fn `UserConstructionScript`)