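; BP_LocustSpawner is a trigger actor that spawns a formation of BP_Locust enemies when a player-controlled pawn overlaps it, unless disabled.
; A delayed for-loop macro staggers child-actor spawns at a ring radius, assigning each locust an alternating roll by index parity.
; Each locust's AI controller receives its formation index, count and a shared start time one second after the final spawn.
; Ending overlap with a BP_Mine destroys the spawner.
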(event `self.ReceiveActorBeginOverlap`
  (params (OtherActor :type "Actor Object Reference"))
  (if (not (`self.bDisableLocusts`))
    ;[1 1 1] if pawn is player controlled, spawn locust(s)
    (bind _aspawn (cast `Pawn` OtherActor))
    (if (`Pawn.IsPlayerControlled` _aspawn)
      (`self.SpawnLocusts`))))

(event `SpawnLocusts`
  ;[1 1 1] get time that the final locust in this formation is created
  (set `self.FormationStartTime` (+ (* (`self.SpawnDelay`) (`KismetMathLibrary.Conv_IntToDouble` (- (`self.LocustCount`) 1))) (`KismetSystemLibrary.GetGameTimeInSeconds`) 1.0))
  ;[1 1 1] Full Circle Spawning
  (bind _index (`self.ForLoopDelay` 0 (- (`self.LocustCount`) 1) (`self.SpawnDelay`))
    (:`LoopBody`
      (bind _returnvalue (`AddComponent|NODE_AddChildActorComponent-0` :`RelativeTransform` (`KismetMathLibrary.MakeTransform` (`KismetMathLibrary.RotateAngleAxis` (`KismetMathLibrary.MakeVector` 0.0 0.0 (`self.RingRadius`)) 0.0 (1.0 0.0 0.0)))))
      (`ChildActorComponent.SetChildActorClass` _returnvalue "/Game/RacingGame/Enemies/Locust/BP_Locust.BP_Locust_C")
      (`|ExecutionSequence`
        (:`then_0`
          (bind _childactor (`ChildActorComponent.ChildActor` _returnvalue))
          (bind _asbp_locust (cast `/Game/RacingGame/Enemies/Locust/BP_Locust` _childactor))
          (set `/Game/RacingGame/Enemies/Locust/BP_Locust.DesiredRoll` (`self.Get Locust Desired Roll` _index) _asbp_locust))
        (:`then_1`
          (bind _asbp_locust_controller (cast `/Game/RacingGame/Enemies/Locust/BP_LocustController` (`AIBlueprintHelperLibrary.GetAIController` _childactor)))
          (set `/Game/RacingGame/Enemies/Locust/BP_LocustController.FormationPosition` _index _asbp_locust_controller)
          (set `/Game/RacingGame/Enemies/Locust/BP_LocustController.FormationStartTime` (`self.FormationStartTime`) _asbp_locust_controller)
          (set `/Game/RacingGame/Enemies/Locust/BP_LocustController.FormationCount` (`self.LocustCount`) _asbp_locust_controller))))))

(event `self.ReceiveActorEndOverlap`
  (params (OtherActor :type "Actor Object Reference"))
  ;[1 1 1] mines kill, FX are on mine blueprint
  (cast `/Game/RacingGame/Interactables/Mine/BP_Mine` OtherActor)
  (`self.K2_DestroyActor`))

(fn `Get Locust Desired Roll`
  (params (Index :type Integer))
  (returns (DesiredRoll :type "Float (double-precision)"))
  (bind _returnvalue (/ 180.0 (`KismetMathLibrary.Conv_IntToDouble` (`self.LocustCount`))))
  (bind _returnvalue_2 (* (`KismetMathLibrary.Conv_IntToDouble` Index) _returnvalue))
  (return (`KismetMathLibrary.SelectFloat` (- 180.0 _returnvalue_2) (+ _returnvalue_2 -180.0 _returnvalue) (`self.IsEvenInt` Index))))

(fn `UserConstructionScript`)